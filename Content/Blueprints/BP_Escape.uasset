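; BP_Escape is the exit door of a stealth game, which opens only once every collectable has been gathered.
; A Box overlap shows and hides a Widget as actors enter and leave.
; Interact reads CollectablesLeft from GM_StealthGameMode: at zero it plays a sound and a timeline swings the Door's yaw open, otherwise it plays a ping sound.
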(event OnComponentBeginOverlap(Box)
  (params (OverlappedComponent :type Primitive%20Component%20Object%20Reference) (OtherActor :type Actor%20Object%20Reference) (OtherComp :type Primitive%20Component%20Object%20Reference) (OtherBodyIndex :type Integer) (bFromSweep :type Boolean) (SweepResult :type Hit%20Result%20Structure%20%28by%20ref%29))
  (Rendering|SetVisibility (Variables|Default|GetWidget) true false))

(event OnComponentEndOverlap(Box)
  (params (OverlappedComponent :type Primitive%20Component%20Object%20Reference) (OtherActor :type Actor%20Object%20Reference) (OtherComp :type Primitive%20Component%20Object%20Reference) (OtherBodyIndex :type Integer))
  (Rendering|SetVisibility (Variables|Default|GetWidget) false false))

(event EventBeginPlay)

(event Collision|EventActorBeginOverlap
  (params (OtherActor :type Actor%20Object%20Reference)))

(event EventTick
  (params (DeltaSeconds :type Float%20%28single-precision%29)))

(event EventInteract
  (bind _asgm_stealth_game_mode (Utilities|Casting|CastToGM_StealthGameMode (Game|GetGameMode)))
  (if (== (Variables|/Game/Blueprints/GameMode/GM_StealthGameMode.GM_StealthGameMode_C|GetCollectablesLeft _asgm_stealth_game_mode) 0)
    (Audio|PlaySoundatLocation "/Engine/VREditor/Sounds/VR_shep_scale_down_03_Cue.VR_shep_scale_down_03_Cue" "0, 0, 0" "0, 0, 0" 1.0 1.0 0.0 0 0 0 0)
    (bind _doortimeline (Timeline|DoorTimeline Play)
      (:Update
        (Transformation|SetRelativeRotation (Variables|Default|GetDoor) (Math|Rotator|MakeRotator 0.0 0.0 (Math|Float|Lerp 0.0 -9e+01 _doortimeline)) false false)))
    (else
      (Audio|PlaySoundatLocation "/Engine/EngineSounds/1kSineTonePing.1kSineTonePing" "0, 0, 0" "0, 0, 0" 1.0 1.0 0.0 0 0 0 0))))

(fn ConstructionScript)