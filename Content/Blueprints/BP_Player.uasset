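; BP_Player is the player character for a stealth game with guards, detection meter, timer and jewel pickup.
; Enhanced Input drives movement, timeline-blended crouching with headroom checks, rolling, camera switching, flashlight and pausing.
; Interact messages overlapping actors through BPI_Interact and performs motion-warped takedowns on BPI_Guard actors.
; Mantling uses stepped sphere traces to find ledges, then motion-warps a 1m or 2m montage while in Flying mode.
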(event Custom|Ragdoll
  (Physics|SetSimulatePhysics (Variables|Character|GetMesh) false)
  (Input|DisableInput 0))

(event Custom|EquipJewel
  (Rendering|SetVisibility (Variables|Default|GetJewel) true false)
  (Variables|Default|SetHasJewel true))

(event Custom|GoToStart
  (bind _returnvalue (Actor|GetActorOfClass "/Script/Engine.PlayerStart"))
  (Transformation|SetActorLocation (Transformation|GetActorLocation _returnvalue) false false))

(event Input|EnhancedActionEvents|EnhancedInputActionIA_Move
  (params (ActionValue :type Vector%202D%20Structure) (ElapsedSeconds :type Float%20%28double-precision%29) (TriggeredSeconds :type Float%20%28double-precision%29) (InputAction :type Input%20Action%20Object%20Reference :default "/Game/Input/IA_Move.IA_Move"))
  (bind _returnvalue (Pawn|GetControlRotation :!class /Script/Engine.Pawn))
  ;[1 1 1] Input and Movement
  ;;[1 1 1] Character Movement
  (Pawn|Input|AddMovementInput (Math|Vector|GetRightVector (Math|Rotator|MakeRotator (.roll _returnvalue) 0.0 (.yaw _returnvalue))) (.x ActionValue) false)
  (Pawn|Input|AddMovementInput (Math|Vector|GetForwardVector (Math|Rotator|MakeRotator 0.0 0.0 (.yaw (Pawn|GetControlRotation :!class /Script/Engine.Pawn)))) (.y ActionValue) false))

(event Input|EnhancedActionEvents|EnhancedInputActionIA_Look
  (params (ActionValue :type Vector%202D%20Structure) (ElapsedSeconds :type Float%20%28double-precision%29) (TriggeredSeconds :type Float%20%28double-precision%29) (InputAction :type Input%20Action%20Object%20Reference :default "/Game/Input/IA_Look.IA_Look"))
  ;[1 1 1] Input and Movement
  ;;[1 1 1] Look with mouse and inverted
  (Pawn|Input|AddControllerYawInput (.x ActionValue))
  (Pawn|Input|AddControllerPitchInput (* (.y ActionValue) -1.0)))

(event Input|EnhancedActionEvents|EnhancedInputActionIA_JumpPlayer
  (params (ActionValue :type Boolean) (ElapsedSeconds :type Float%20%28double-precision%29) (TriggeredSeconds :type Float%20%28double-precision%29) (InputAction :type Input%20Action%20Object%20Reference :default "/Game/Input/IA_JumpPlayer.IA_JumpPlayer"))
  (:Started
    (Character|Jump))
  (:Canceled
    (Character|StopJumping :!label _label))
  (:Completed
    (goto _label)))

(event Input|EnhancedActionEvents|EnhancedInputActionIA_Interact
  (params (ActionValue :type Boolean) (ElapsedSeconds :type Float%20%28double-precision%29) (TriggeredSeconds :type Float%20%28double-precision%29) (InputAction :type Input%20Action%20Object%20Reference :default "/Game/Input/IA_Interact.IA_Interact"))
  ;[1 1 1] Interact
  (:Started
    (Utilities|FlowControl|Sequence
      (:then_0
        (for _array_element (Collision|GetOverlappingActors 0 :!class /Script/Engine.Actor)
          (if (Utilities|DoesObjectImplementInterface _array_element "/Game/Blueprints/BPI_Interact.BPI_Interact_C")
            (Class|BPIInteract|Interact(Message) _array_element))))
      (:then_1
        (for _array_element_2 (Collision|GetOverlappingActors 0 :!class /Script/Engine.Actor)
          (if (Utilities|DoesObjectImplementInterface _array_element_2 "/Game/Blueprints/BPI_Guard.BPI_Guard_C")
            (bind (_refpose _rotation _cantakedown _aiactor) (Class|BPIGuard|Takedown(Message) _array_element_2))
            (if _cantakedown
              (Animation|Montage|PlayMontage (Variables|Character|GetMesh) "/Game/Characters/Player/Takedown_Animations/Takedown_Attacker_Montage.Takedown_Attacker_Montage"
                (:then
                  (Class|MotionWarpingComponent|AddorUpdateWarpTarget (Variables|Default|GetMotionWarping) (Utilities|Struct|MakeMotionWarpingTarget "Takedown" _refpose _rotation 0 "None" false "0.000000,0.000000,0.000000" "0.000000,0.000000,0.000000"))
                  (Collision|IgnoreActorwhenMoving (Variables|Character|GetMesh) _aiactor true))))))))))

(event Input|EnhancedActionEvents|EnhancedInputActionIA_Crouch
  (params (ActionValue :type Boolean) (ElapsedSeconds :type Float%20%28double-precision%29) (TriggeredSeconds :type Float%20%28double-precision%29) (InputAction :type Input%20Action%20Object%20Reference :default "/Game/Input/IA_Crouch.IA_Crouch"))
  (bind _charactermovement (Variables|Character|GetCharacterMovement))
  ;[1 1 1] Crouch
  (:Started
    (if (not (Variables|Default|GetCrouched))
      (Variables|Default|SetCrouched true)
      (Variables|/Script/Engine.CharacterMovementComponent|SetMaxWalkSpeed _charactermovement 3.5e+02)
      (Utilities|FlowControl|Sequence
        (:then_0
          (bind _armlength (Timeline|CrouchZoom Play)
            (:Update
              (Variables|/Script/Engine.SpringArmComponent|SetTargetArmLength (Variables|Default|GetSpringArm) (Math|Float|Lerp 6e+02 7.5e+02 _armlength)))))
        (:then_1
          (bind _capsuleheight (Timeline|CapsuleHeight Play)
            (:Update
              (Components|Capsule|SetCapsuleHalfHeight (Variables|Collision|GetCapsuleComponent) (Math|Float|Lerp 88.0 5e+01 _capsuleheight) true)
              (Transformation|SetRelativeLocation (Variables|Character|GetMesh) (Math|Vector|MakeVector 0.0 0.0 (Math|Float|Lerp -89.0 -59.0 _capsuleheight)) false false)))))
      (else
        (bind _hit_ (CallFunction|UncrouchObstacleDetection))
        (if (not _hit_)
          (Variables|Default|SetCrouched false)
          (Variables|/Script/Engine.CharacterMovementComponent|SetMaxWalkSpeed _charactermovement 6e+02)
          (Utilities|FlowControl|Sequence
            (:then_0
              (Timeline|CrouchZoom Reverse))
            (:then_1
              (Timeline|CapsuleHeight Reverse))))))))

(event Input|EnhancedActionEvents|EnhancedInputActionIA_Roll
  (params (ActionValue :type Boolean) (ElapsedSeconds :type Float%20%28double-precision%29) (TriggeredSeconds :type Float%20%28double-precision%29) (InputAction :type Input%20Action%20Object%20Reference :default "/Game/Input/IA_Roll.IA_Roll"))
  ;[1 1 1] Dodge/Roll
  (:Started
    (if (not (Variables|Default|GetIsDodging))
      (Animation|Montage|PlayMontage (Variables|Character|GetMesh) "/Game/Characters/Player/Roll/Roll_Montage.Roll_Montage"
        (:then
          (Variables|Default|SetIsDodging true))
        (:OnCompleted
          (Variables|Default|SetIsDodging false))))))

(event Input|EnhancedActionEvents|EnhancedInputActionIA_Mantle
  (params (ActionValue :type Boolean) (ElapsedSeconds :type Float%20%28double-precision%29) (TriggeredSeconds :type Float%20%28double-precision%29) (InputAction :type Input%20Action%20Object%20Reference :default "/Game/Input/IA_Mantle.IA_Mantle"))
  (bind _returnvalue (Transformation|GetActorForwardVector))
  (:Started
    (if (and (not (Variables|Default|GetMantling)) (not (AI|Components|NavMovement|IsFalling (Variables|Character|GetCharacterMovement))))
      (bind _index (Utilities|FlowControl|ForLoopwithBreak 0 (Math|Integer|SelectInt 7 4 (Variables|Default|GetCrouched)) :!label _label)
        (:LoopBody
          (bind (_outhit _returnvalue_2) (Collision|SphereTraceByChannel (+ (Transformation|GetActorLocation) (Math|Vector|MakeVector 0.0 0.0 (* _index 30))) (+ (+ (Transformation|GetActorLocation) (Math|Vector|MakeVector 0.0 0.0 (* _index 30))) (* (Math|Vector|GetForwardVector (Transformation|GetActorRotation)) 1.2e+02)) 7.0 "TraceTypeQuery1" false 0 "None"))
          (if (not _returnvalue_2)
            (Utilities|FlowControl|Sequence
              (:then_0
                (if (!= _index 0)
                  (bind _index_2 (Utilities|FlowControl|ForLoopwithBreak 0 4 :!label _label_2)
                    (:LoopBody
                      (bind (_outhit_2 _returnvalue_3) (Collision|SphereTraceByChannel (+ (Transformation|GetActorLocation) (Math|Vector|MakeVector (* (* _index_2 20) (.x _returnvalue)) (* (.y _returnvalue) (* _index_2 20)) 2e+02)) (+ (+ (Transformation|GetActorLocation) (Math|Vector|MakeVector (* (* _index_2 20) (.x _returnvalue)) (* (.y _returnvalue) (* _index_2 20)) 2e+02)) (* (Transformation|GetActorUpVector) -2e+02)) 7.0 "TraceTypeQuery1" false 0 "None"))
                      (if _returnvalue_3
                        (Utilities|FlowControl|Sequence
                          (:then_0
                            (Class|MotionWarpingComponent|AddorUpdateWarpTarget (Variables|Default|GetMotionWarping) (Utilities|Struct|MakeMotionWarpingTarget "Mantle" (+ (.Location (Collision|BreakHitResult _outhit_2)) "0.000000,0.000000,-3.000000") (Transformation|GetActorRotation) 0 "None" false "0.000000,0.000000,0.000000" "0.000000,0.000000,0.000000"))
                            (if (> (Math|Vector|Distance(Vector) (.Location (Collision|BreakHitResult _outhit_2)) (Transformation|GetWorldLocation (Variables|Character|GetMesh))) 2e+02)
                              (Development|PrintString "2m")
                              (Animation|Montage|PlayMontage (Variables|Character|GetMesh) "/Game/Characters/Player/Mantling/Mantling_2M_Montage.Mantling_2M_Montage"
                                (:then
                                  (Pawn|Components|CharacterMovement|SetMovementMode (Variables|Character|GetCharacterMovement) "MOVE_Flying" 0 :!label _label_3)
                                  (Variables|Default|SetMantling true)
                                  (if (Variables|Default|GetCrouched)
                                    (Components|Capsule|SetCapsuleHalfHeight (Variables|Collision|GetCapsuleComponent) 88.0 true)
                                    (Transformation|SetRelativeLocation (Variables|Character|GetMesh) "0.000000,0.000000,-89.000000" false false)))
                                (:OnCompleted
                                  (Variables|Default|SetMantling false :!label _label_4)
                                  (Pawn|Components|CharacterMovement|SetMovementMode (Variables|Character|GetCharacterMovement) "MOVE_Walking" 0)
                                  (if (Variables|Default|GetCrouched)
                                    (bind _capsuleheight (Timeline|Timeline Play)
                                      (:Update
                                        (Components|Capsule|SetCapsuleHalfHeight (Variables|Collision|GetCapsuleComponent) (Math|Float|Lerp 88.0 5e+01 _capsuleheight) true)
                                        (Transformation|SetRelativeLocation (Variables|Character|GetMesh) (Math|Vector|MakeVector 0.0 0.0 (Math|Float|Lerp -89.0 -59.0 _capsuleheight)) false false))))))
                              (else
                                (Development|PrintString "1m")
                                (Animation|Montage|PlayMontage (Variables|Character|GetMesh) "/Game/Characters/Player/Mantling/Mantling_1M_Montage.Mantling_1M_Montage"
                                  (:then
                                    (goto _label_3))
                                  (:OnCompleted
                                    (goto _label_4))))))
                          (:then_1
                            (goto _label_2 Break))))))))
              (:then_1
                (goto _label Break)))))))))

(event Input|EnhancedActionEvents|EnhancedInputActionIA_PauseGame
  (params (ActionValue :type Boolean) (ElapsedSeconds :type Float%20%28double-precision%29) (TriggeredSeconds :type Float%20%28double-precision%29) (InputAction :type Input%20Action%20Object%20Reference :default "/Game/Input/IA_PauseGame.IA_PauseGame"))
  (bind _returnvalue (Game|GetPlayerController 0))
  (bind _returnvalue_2 (Game|GetPlayerController 0))
  (:Started
    (if (not (Variables|Default|GetPaused))
      (Variables|Default|SetPaused true)
      (bind _returnvalue_3 (UserInterface|CreateWidget "/Game/UI/WB_PausedMenu.WB_PausedMenu_C"))
      (bind _output_get (Variables|Default|SetPausedMenuWidget _returnvalue_3))
      (UserInterface|Viewport|AddtoViewport _output_get 0)
      (Variables|/Script/Engine.PlayerController|SetbShowMouseCursor _returnvalue_2 true)
      (Input|SetInputModeGameandUI _returnvalue_2 (Variables|Default|GetPausedMenuWidget) "DoNotLock" true false)
      (Game|SetGamePaused true)
      (else
        (bind _pausedmenuwidget (Variables|Default|GetPausedMenuWidget)
          (:then
            (Widget|RemovefromParent _pausedmenuwidget)
            (Variables|Default|SetPausedMenuWidget 0)
            (Variables|Default|SetPaused false)
            (Variables|/Script/Engine.PlayerController|SetbShowMouseCursor _returnvalue false)
            (Input|SetInputModeGameOnly _returnvalue false)
            (Game|SetGamePaused false))
          (:else))))))

(event Input|EnhancedActionEvents|EnhancedInputActionIA_Interact
  (params (ActionValue :type Boolean) (ElapsedSeconds :type Float%20%28double-precision%29) (TriggeredSeconds :type Float%20%28double-precision%29) (InputAction :type Input%20Action%20Object%20Reference :default "/Game/Input/IA_Interact.IA_Interact"))
  (:Started
    (bind _array_element (Utilities|Array|ForEachLoopwithBreak (Collision|GetOverlappingActors "BP_Player_C" :!class /Script/Engine.Actor) :!label _label)
      (:LoopBody
        (if (Utilities|DoesObjectImplementInterface _array_element "/Game/Blueprints/BPI_Interact.BPI_Interact_C")
          (Class|BPIInteract|Interact(Message) _array_element)
          (goto _label Break))))))

(event Input|EnhancedActionEvents|EnhancedInputActionIA_FirstPersonCamera
  (params (ActionValue :type Boolean) (ElapsedSeconds :type Float%20%28double-precision%29) (TriggeredSeconds :type Float%20%28double-precision%29) (InputAction :type Input%20Action%20Object%20Reference :default "/Game/Input/IA_FirstPersonCamera.IA_FirstPersonCamera"))
  (Utilities|FlowControl|FlipFlop
    (:A
      (Components|Activation|SetActive (Variables|Default|GetFirstPersonCamera) true false)
      (Components|Activation|SetActive (Variables|Default|GetCamera) false false)
      (Variables|Default|SetbUseControllerRotationYaw true))
    (:B
      (Components|Activation|SetActive (Variables|Default|GetFirstPersonCamera) false false)
      (Components|Activation|SetActive (Variables|Default|GetCamera) true false)
      (Variables|Default|SetbUseControllerRotationYaw false))))

(event Input|EnhancedActionEvents|EnhancedInputActionIA_FlashLight
  (params (ActionValue :type Boolean) (ElapsedSeconds :type Float%20%28double-precision%29) (TriggeredSeconds :type Float%20%28double-precision%29) (InputAction :type Input%20Action%20Object%20Reference :default "/Game/Input/IA_FlashLight.IA_FlashLight"))
  (bind _spotlight (Variables|Default|GetSpotLight))
  (bind _returnvalue (Transformation|GetWorldLocation _spotlight))
  (:Started
    (Utilities|FlowControl|FlipFlop
      (:A
        (Audio|PlaySoundatLocation "/Engine/VREditor/Sounds/UI/Flashlight_Switch.Flashlight_Switch" _returnvalue "0, 0, 0" 1.0 1.0 0.0 0 0 0 0)
        (Utilities|FlowControl|Delay 0.15)
        (Rendering|SetVisibility _spotlight true false)
        (Variables|Default|SetFlashLight true))
      (:B
        (Audio|PlaySoundatLocation "/Engine/VREditor/Sounds/UI/Flashlight_Switch.Flashlight_Switch" _returnvalue "0, 0, 0" 1.0 1.0 0.0 0 0 0 0)
        (Rendering|SetVisibility _spotlight false false)
        (Variables|Default|SetFlashLight false)))))

(event EventBeginPlay
  ;[1 1 1] Input and Movement
  (Input|AddMappingContext (PlayerController|LocalPlayerSubsystems|GetEnhancedInputLocalPlayerSubsystem (Game|GetPlayerController 0)) "/Game/Input/IMC_PlayerInput.IMC_PlayerInput" 0 "(bIgnoreAllPressedKeysUntilRelease=True,bForceImmediately=False,bNotifyUserSettings=False)")
  (bind _returnvalue (Game|GetCurrentLevelName true))
  (if (Utilities|Enum|NotEqual(Enum) _returnvalue "MainMenu")
    (bind _returnvalue_2 (UserInterface|CreateWidget "/Game/UI/WB_DetectionMeter.WB_DetectionMeter_C"))
    (bind _output_get (Variables|Default|SetDetectionMeterWidget _returnvalue_2))
    (UserInterface|Viewport|AddtoViewport _output_get 0)
    (bind _returnvalue_3 (UserInterface|CreateWidget "/Game/UI/WB_Timer.WB_Timer_C"))
    (bind _output_get_2 (Variables|Default|SetTimerWidget _returnvalue_3))
    (UserInterface|Viewport|AddtoViewport _output_get_2 0)))

(event Collision|EventActorBeginOverlap
  (params (OtherActor :type Actor%20Object%20Reference))
  ;[1 1 1] Crouch
)

(event EventTick
  (params (DeltaSeconds :type Float%20%28single-precision%29)))

(fn ConstructionScript
  (Components|SkinnedMesh|SetLeaderPoseComponent (Variables|Default|GetFace) (Variables|Character|GetMesh) false false))

(fn UncrouchObstacleDetection
  (bind _returnvalue (Transformation|GetActorLocation))
  (bind _returnvalue_2 (Collision|SphereTraceByChannel _returnvalue (+ _returnvalue (* (Math|Vector|GetUpVector (Transformation|GetActorRotation)) 115.0)) 15.0 "TraceTypeQuery1" false 0 "None"))
  (return _returnvalue_2))