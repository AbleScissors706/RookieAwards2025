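; BP_Sensor is a sensor actor that raises the alarm when it detects the player, then restarts the level.
; DetectPlayer fires once for a Player-tagged actor, playing an attenuated camera shutter sound and starting the first BP_Alarm found.
; A timeline drives a point light flash.
; Its Update also feeds a delay before the Restartlevel console command, a fallback for when no enemies are present.
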(event Custom|DetectPlayer
  (params (ActorDetected :type Actor%20Object%20Reference))
  (if (and (Actor|ActorHasTag ActorDetected "Player") (not (Variables|Default|GetHasDetected)))
    (Variables|Default|SetHasDetected true)
    (Audio|PlaySoundatLocation "/Engine/VREditor/Sounds/UI/Camera_Shutter.Camera_Shutter" (Transformation|GetActorLocation) "0, 0, 0" 1.0 1.0 0.0 "/Game/Audio/Grunts/SA_Sensor.SA_Sensor" 0 0 0)
    (bind _returnvalue (Actor|GetActorOfClass "/Game/Blueprints/Sensor_Alarms/BP_Alarm.BP_Alarm_C"))
    (Default|StartAlarm _returnvalue)
    (bind _intensity_of_light (Timeline|PointLightTimeline Play)
      (:Update
        (Rendering|Components|Light|SetIntensity (Variables|Default|GetPointLight) (Math|Float|Lerp 0.0 1e+05 _intensity_of_light))
        ;[0.15 0.15 0.15 0.5] added this for player when caught by bar sensor it has a delay of xTime so that if there is no Enemies the game restarts/little bug fix
        (Utilities|FlowControl|Delay 7.0)
        (Development|ExecuteConsoleCommand "Restartlevel" 0)))))

(event EventBeginPlay)

(event Collision|EventActorBeginOverlap
  (params (OtherActor :type Actor%20Object%20Reference)))

(event EventTick
  (params (DeltaSeconds :type Float%20%28single-precision%29)))

(fn ConstructionScript)