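; BP_Sensor_Bar is a sensor-bar alarm hazard that restarts the level after something enters its trigger.
; Trigger overlap passes the actor to DetectPlayer, defined outside this file, then waits a fixed delay and runs the Restartlevel console command.
; Interact toggles the sensor via an Activated flag, switching actor collision and the visibility of Bars and its children together.
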(event OnComponentBeginOverlap(Trigger)
  (params (OverlappedComponent :type Primitive%20Component%20Object%20Reference) (OtherActor :type Actor%20Object%20Reference) (OtherComp :type Primitive%20Component%20Object%20Reference) (OtherBodyIndex :type Integer) (bFromSweep :type Boolean) (SweepResult :type Hit%20Result%20Structure%20%28by%20ref%29))
  (CallFunction|DetectPlayer OtherActor)
  (Utilities|FlowControl|Delay 5.0)
  (Development|ExecuteConsoleCommand "Restartlevel" 0))

(event EventBeginPlay
  (|CallParentFunction) ; This node is disabled and will not be called.\nDrag off pins to build functionality.
)

(event Collision|EventActorBeginOverlap
  (params (OtherActor :type Actor%20Object%20Reference))
  (|CallParentFunction OtherActor) ; This node is disabled and will not be called.\nDrag off pins to build functionality.
)

(event EventTick
  (params (DeltaSeconds :type Float%20%28single-precision%29))
  (|CallParentFunction DeltaSeconds) ; This node is disabled and will not be called.\nDrag off pins to build functionality.
)

(event EventInteract
  (if (not (Variables|Default|GetActivated))
    (Collision|SetActorEnableCollision true)
    (Rendering|SetVisibility (Variables|Default|GetBars) true true)
    (Variables|Default|SetActivated true)
    (else
      (Collision|SetActorEnableCollision false)
      (Rendering|SetVisibility (Variables|Default|GetBars) false true)
      (Variables|Default|SetActivated false))))

(fn ConstructionScript
  (|CallParentFunction))