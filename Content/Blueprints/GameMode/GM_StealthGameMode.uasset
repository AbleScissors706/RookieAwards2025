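; Game mode for a stealth game that manages music, rain ambience and the player's capture sequence.
; BeginPlay fades in music and a rain loop and sets game-only input; SwitchMusicToEscaping swaps to escape music.
; Captured shows the cursor and an animated captured widget.
; Only when escape music is valid does Captured also fade it and the BP_Alarm sound, play a caught sound and ragdoll BP_Player.
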(event Custom|Captured
  (bind _returnvalue (Game|GetPlayerController 0))
  (Variables|/Script/Engine.PlayerController|SetbShowMouseCursor _returnvalue true)
  (Input|SetInputModeGameandUI _returnvalue 0 "DoNotLock" true false)
  (bind _returnvalue_2 (UserInterface|CreateWidget "/Game/UI/WB_Captured.WB_Captured_C"))
  (bind _output_get (Variables|Default|SetCapturedWidget _returnvalue_2))
  (UserInterface|Viewport|AddtoViewport _output_get 0)
  (Default|FadeAnimation (Variables|Default|GetCapturedWidget))
  (bind _escapingmusic (Variables|Default|GetEscapingMusic)
    (:then
      (Audio|Components|Audio|FadeOut _escapingmusic 0.3 0.0 "Linear" :!class /Script/Engine.AudioComponent)
      (Audio|PlaySound2D "/Game/Audio/Effects/Caught.Caught" 1.0 1.0 0.0 0 0)
      (bind _returnvalue_3 (Actor|GetActorOfClass "/Game/Blueprints/Sensor_Alarms/BP_Alarm.BP_Alarm_C"))
      (Audio|Components|Audio|FadeOut (Variables|/Game/Blueprints/Sensor_Alarms/BP_Alarm.BP_Alarm_C|GetAlarmSound _returnvalue_3) 0.5 0.0 "Linear" :!class /Script/Engine.AudioComponent)
      (bind _asbp_player (Utilities|Casting|CastToBP_Player (Game|GetPlayerCharacter 0)))
      (Default|Ragdoll _asbp_player))
    (:else)))

(event Custom|SwitchMusicToEscaping
  (Audio|Components|Audio|FadeOut (Variables|Default|GetMusic) 0.3 0.0 "Linear" :!class /Script/Engine.AudioComponent)
  (bind _returnvalue (Audio|SpawnSound2D "/Game/Audio/Music/Escaping.Escaping" 0.5 1.0 0.0 0))
  (Variables|Default|SetEscapingMusic _returnvalue))

(event EventBeginPlay
  (bind _returnvalue (Game|GetPlayerController 0))
  (bind _returnvalue_2 (Audio|SpawnSound2D "/Game/Audio/Music/Music.Music" 0.3 1.0 0.0 0))
  (bind _output_get (Variables|Default|SetMusic _returnvalue_2))
  (Audio|Components|Audio|FadeIn _output_get 0.3 1.0 0.0 "Linear" :!class /Script/Engine.AudioComponent)
  (bind _returnvalue_3 (Audio|SpawnSound2D "/Game/Audio/Effects/Rain_Loop.Rain_Loop" 0.5 1.0 0.0 0))
  (bind _output_get_2 (Variables|Default|SetRainLoop _returnvalue_3))
  (Audio|Components|Audio|FadeIn _output_get_2 1.0 1.0 0.0 "Linear" :!class /Script/Engine.AudioComponent)
  (Variables|/Script/Engine.PlayerController|SetbShowMouseCursor _returnvalue false)
  (Input|SetInputModeGameOnly _returnvalue false))

(event EventTick
  (params (DeltaSeconds :type Float%20%28single-precision%29)))

(fn ConstructionScript)