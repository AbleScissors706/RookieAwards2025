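; BP_LevelTransition is a door that swings open on approach and moves the player to another level.
; Overlapping DoorOpenCollision plays a timeline that yaws DoorMesh open, and ending the overlap reverses it, with open and close sounds played at world origin.
; When BP_Player enters LevelTransitionCollision, it opens the level named by MapTransition unless that name is None.
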(event OnComponentBeginOverlap(DoorOpenCollision)
  (params (OverlappedComponent :type Primitive%20Component%20Object%20Reference) (OtherActor :type Actor%20Object%20Reference) (OtherComp :type Primitive%20Component%20Object%20Reference) (OtherBodyIndex :type Integer) (bFromSweep :type Boolean) (SweepResult :type Hit%20Result%20Structure%20%28by%20ref%29))
  (Audio|PlaySoundatLocation "/Engine/VREditor/Sounds/UI/Dockable_Window_Open.Dockable_Window_Open" "0, 0, 0" "0, 0, 0" 1.0 1.0 0.0 0 0 0 0)
  (bind _doortimeline (Timeline|Timeline Play)
    (:Update
      (Transformation|SetRelativeRotation (Variables|Default|GetDoorMesh) (Math|Rotator|MakeRotator 0.0 0.0 (Math|Float|Lerp 0.0 1.1e+02 _doortimeline)) false false))))

(event OnComponentEndOverlap(DoorOpenCollision)
  (params (OverlappedComponent :type Primitive%20Component%20Object%20Reference) (OtherActor :type Actor%20Object%20Reference) (OtherComp :type Primitive%20Component%20Object%20Reference) (OtherBodyIndex :type Integer))
  (Audio|PlaySoundatLocation "/Engine/VREditor/Sounds/UI/Dockable_Window_Close.Dockable_Window_Close" "0, 0, 0" "0, 0, 0" 1.0 1.0 0.0 0 0 0 0)
  (bind _doortimeline (Timeline|Timeline Reverse)
    (:Update
      (Transformation|SetRelativeRotation (Variables|Default|GetDoorMesh) (Math|Rotator|MakeRotator 0.0 0.0 (Math|Float|Lerp 0.0 1.1e+02 _doortimeline)) false false))))

(event OnComponentBeginOverlap(LevelTransitionCollision)
  (params (OverlappedComponent :type Primitive%20Component%20Object%20Reference) (OtherActor :type Actor%20Object%20Reference) (OtherComp :type Primitive%20Component%20Object%20Reference) (OtherBodyIndex :type Integer) (bFromSweep :type Boolean) (SweepResult :type Hit%20Result%20Structure%20%28by%20ref%29))
  (Utilities|Casting|CastToBP_Player OtherActor)
  (if (Utilities|Enum|NotEqual(Enum) (Utilities|String|ToString(Name) (Variables|Default|GetMap%20Transition)) "None")
    (Game|OpenLevel(byName) (Variables|Default|GetMap%20Transition))))

(event EventBeginPlay)

(event Collision|EventActorBeginOverlap
  (params (OtherActor :type Actor%20Object%20Reference)))

(event EventTick
  (params (DeltaSeconds :type Float%20%28single-precision%29)))

(fn ConstructionScript)