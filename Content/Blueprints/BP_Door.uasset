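; BP_Door is a key-locked door that swings open and closed on interaction.
; PickUpKey sets HasKey, and Interact does nothing until that flag is true.
; A FlipFlop then alternates between playing and reversing DoorTimeline, which lerps the door's relative yaw to swing it open or shut.
; Each toggle plays an open or close sound at the world origin rather than at the door.
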(event EventBeginPlay)

(event Collision|EventActorBeginOverlap
  (params (OtherActor :type Actor%20Object%20Reference)))

(event EventTick
  (params (DeltaSeconds :type Float%20%28single-precision%29)))

(event EventInteract
  (if (Variables|Default|GetHasKey)
    (Utilities|FlowControl|FlipFlop
      (:A
        (Audio|PlaySoundatLocation "/Engine/VREditor/Sounds/UI/Dockable_Window_Open.Dockable_Window_Open" "0, 0, 0" "0, 0, 0" 1.0 1.0 0.0 0 0 0 0)
        (bind _doortimeline (Timeline|DoorTimeline Play)
          (:Update
            (Transformation|SetRelativeRotation (Variables|Default|GetDoor) (Math|Rotator|MakeRotator 0.0 0.0 (Math|Float|Lerp 0.0 1.1e+02 _doortimeline)) false false))))
      (:B
        (Audio|PlaySoundatLocation "/Engine/VREditor/Sounds/UI/Dockable_Window_Close.Dockable_Window_Close" "0, 0, 0" "0, 0, 0" 1.0 1.0 0.0 0 0 0 0)
        (Timeline|DoorTimeline Reverse)))))

(event EventPickUpKey
  (Variables|Default|SetHasKey true))

(fn ConstructionScript)