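; BP_Dummy is a character that serves as a takedown victim for the player.
; Its TakedownRadius overlaps show the prompt widget to a Player-tagged actor while it is alive, and hide it on exit.
; If CanTakedown is set, Takedown plays the victim montage, marks it dead and returns the REF location and actor rotation.
; A delayed event then ragdolls the mesh and disables movement.
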(event OnComponentBeginOverlap(TakedownRadius)
  (params (OverlappedComponent :type Primitive%20Component%20Object%20Reference) (OtherActor :type Actor%20Object%20Reference) (OtherComp :type Primitive%20Component%20Object%20Reference) (OtherBodyIndex :type Integer) (bFromSweep :type Boolean) (SweepResult :type Hit%20Result%20Structure%20%28by%20ref%29))
  (if (and (Actor|ActorHasTag OtherActor "Player") (not (Variables|Default|GetDead)))
    (Rendering|SetVisibility (Variables|Default|GetTakedownPromptWidget) true false)))

(event OnComponentEndOverlap(TakedownRadius)
  (params (OverlappedComponent :type Primitive%20Component%20Object%20Reference) (OtherActor :type Actor%20Object%20Reference) (OtherComp :type Primitive%20Component%20Object%20Reference) (OtherBodyIndex :type Integer))
  (if (Actor|ActorHasTag OtherActor "Player")
    (Rendering|SetVisibility (Variables|Default|GetTakedownPromptWidget) false false)))

(event Custom|TakedownRagDoll
  (Utilities|FlowControl|Delay 1.27)
  (Physics|SetSimulatePhysics (Variables|Character|GetMesh) true)
  (Pawn|Components|CharacterMovement|SetMovementMode (Variables|Character|GetCharacterMovement) "MOVE_None" 0))

(event EventBeginPlay)

(event Collision|EventActorBeginOverlap
  (params (OtherActor :type Actor%20Object%20Reference)))

(event EventTick
  (params (DeltaSeconds :type Float%20%28single-precision%29)))

(fn ConstructionScript)

(fn Takedown
  (if (Variables|Default|GetCanTakedown)
    (Animation|PlayAnimMontage "/Game/Characters/Player/Takedown_Animations/Takedown_Victim_Montage.Takedown_Victim_Montage" 1.0 "None")
    (CallFunction|TakedownRagDoll)
    (Rendering|SetVisibility (Variables|Default|GetTakedownPromptWidget) false false)
    (Variables|Default|SetDead true)
    (return (Transformation|GetWorldLocation (Variables|Default|GetREF)) (Transformation|GetActorRotation) (Variables|Default|GetCanTakedown) 0)))