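; BP_Guard is the guard character in a stealth game that can catch the player or be taken down by them.
; An overlap radius shows the takedown prompt; Takedown plays the victim montage, marks guard and AI controller dead, returns a reference pose for alignment, and ragdolls after a delay.
; Catch plays a montage whose notify sphere-traces ahead and reports a captured player to GM_StealthGameMode.
; Run raises walk speed.
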(event OnComponentBeginOverlap(TakedownRadius)
  (params (OverlappedComponent :type Primitive%20Component%20Object%20Reference) (OtherActor :type Actor%20Object%20Reference) (OtherComp :type Primitive%20Component%20Object%20Reference) (OtherBodyIndex :type Integer) (bFromSweep :type Boolean) (SweepResult :type Hit%20Result%20Structure%20%28by%20ref%29))
  (if (and (Actor|ActorHasTag OtherActor "Player") (not (Variables|Default|GetDead)))
    (Rendering|SetVisibility (Variables|Default|GetTakedownPromptWidget) true false)))

(event OnComponentEndOverlap(TakedownRadius)
  (params (OverlappedComponent :type Primitive%20Component%20Object%20Reference) (OtherActor :type Actor%20Object%20Reference) (OtherComp :type Primitive%20Component%20Object%20Reference) (OtherBodyIndex :type Integer))
  (if (Actor|ActorHasTag OtherActor "Player")
    (Rendering|SetVisibility (Variables|Default|GetTakedownPromptWidget) false false)))

(event Custom|TakedownRagDoll
  (Utilities|FlowControl|Delay 1.27)
  (Audio|PlaySoundatLocation "/Engine/VREditor/Sounds/UI/Gizmo_Handle_Clicked.Gizmo_Handle_Clicked" "0, 0, 0" "0, 0, 0" 1.0 1.0 0.0 0 0 0 0)
  (Physics|SetSimulatePhysics (Variables|Character|GetMesh) true)
  (Pawn|Components|CharacterMovement|SetMovementMode (Variables|Character|GetCharacterMovement) "MOVE_None" 0))

(event EventBeginPlay)

(event Collision|EventActorBeginOverlap
  (params (OtherActor :type Actor%20Object%20Reference)))

(event EventTick
  (params (DeltaSeconds :type Float%20%28single-precision%29)))

(event EventRun
  (Variables|/Script/Engine.CharacterMovementComponent|SetMaxWalkSpeed (Variables|Character|GetCharacterMovement) 5e+02))

(event EventCatch
  (bind _returnvalue (Transformation|GetActorLocation))
  (if (not (Variables|Default|GetIsAttacking))
    (Animation|Montage|PlayMontage (Variables|Character|GetMesh) "/Game/Characters/Player/Catch/Catch_Montage.Catch_Montage"
      (:then
        (Variables|Default|SetIsAttacking true))
      (:OnCompleted
        (Variables|Default|SetIsAttacking false))
      (:OnNotifyBegin
        (bind (_outhit _returnvalue_2) (Collision|SphereTraceForObjects _returnvalue (+ _returnvalue (* (Transformation|GetActorForwardVector) 1.2e+02)) 3e+01 (Utilities|Array|MakeArray "ObjectTypeQuery3") false 0 "ForDuration"))
        (if _returnvalue_2
          (if (Actor|ActorHasTag (.HitActor (Collision|BreakHitResult _outhit)) "Player")
            (Utilities|FlowControl|DoOnce false
              (:Completed
                (bind _asgm_stealth_game_mode (Utilities|Casting|CastToGM_StealthGameMode (Game|GetGameMode)))
                (Default|Captured _asgm_stealth_game_mode)))))))))

(fn ConstructionScript)

(fn Takedown
  (if (Variables|Default|GetCanTakedown)
    (Animation|PlayAnimMontage "/Game/Characters/Player/Takedown_Animations/Takedown_Victim_Montage.Takedown_Victim_Montage" 1.0 "None")
    (CallFunction|TakedownRagDoll)
    (Rendering|SetVisibility (Variables|Default|GetTakedownPromptWidget) false false)
    (Variables|Default|SetDead true)
    (bind _asbp_ai_guard (Utilities|Casting|CastToBP_AI_Guard (AI|GetAIController self)))
    (Variables|/Game/AI/BP_AI_Guard.BP_AI_Guard_C|SetDead _asbp_ai_guard true)
    (return (Transformation|GetWorldLocation (Variables|Default|GetREF)) (Transformation|GetActorRotation) (Variables|Default|GetCanTakedown) 0)))